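; BP_Enemy is an enemy that chases the player character and damages it on contact.
; On BeginPlay it runs an AI move toward the player, then repeats after a short delay each time a move finishes.
; Overlaps on its Box component subtract Health directly from BP_TopDownCharacter.
; Tick polls the enemy's own Health and destroys the actor when it runs out.
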(event `self.ReceiveBeginPlay`
  (`|AIMoveTo` self (0.0 0.0 0.0) (`GameplayStatics.GetPlayerCharacter` 0) :!label _label
    (:`then`
      (`KismetSystemLibrary.Delay` 1.0)
      (goto _label))))

(event `self.ReceiveTick`
  (params (DeltaSeconds :type "Float (single-precision)"))
  (if (<= (`self.Health`) 0)
    (`self.K2_DestroyActor`)))

(event `self.Box.OnComponentBeginOverlap`
  (params (OverlappedComponent :type "PrimitiveComponent Object Reference") (OtherActor :type "Actor Object Reference") (OtherComp :type "PrimitiveComponent Object Reference") (OtherBodyIndex :type Integer) (bFromSweep :type Boolean) (SweepResult :type "HitResult Structure (by ref)"))
  (bind _asbp_top_down_character (cast `/Game/Main/Blueprints/BP_TopDownCharacter` OtherActor))
  (set `/Game/Main/Blueprints/BP_TopDownCharacter.Health ` (- (`/Game/Main/Blueprints/BP_TopDownCharacter.Health ` _asbp_top_down_character) 10) _asbp_top_down_character))

(fn `UserConstructionScript`)