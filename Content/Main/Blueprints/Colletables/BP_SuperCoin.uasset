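; BP_SuperCoin is a collectible coin that adds 10 Gold to BP_TopDownCharacter and destroys itself when that character overlaps its Trigger.
; It spins a little every Tick.
; Overlap with the larger MagnetZone component toggles a Magnet flag for that character, and while it is set Tick interpolates the coin toward player character 0 with VInterpTo.
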(event `self.ReceiveBeginPlay`)

(event `self.Trigger.OnComponentBeginOverlap`
  (params (OverlappedComponent :type "PrimitiveComponent Object Reference") (OtherActor :type "Actor Object Reference") (OtherComp :type "PrimitiveComponent Object Reference") (OtherBodyIndex :type Integer) (bFromSweep :type Boolean) (SweepResult :type "HitResult Structure (by ref)"))
  (bind _asbp_top_down_character (cast `/Game/Main/Blueprints/BP_TopDownCharacter` OtherActor))
  (set `/Game/Main/Blueprints/BP_TopDownCharacter.Gold` (+ (`/Game/Main/Blueprints/BP_TopDownCharacter.Gold` _asbp_top_down_character) 10) _asbp_top_down_character)
  (`self.K2_DestroyActor`))

(event `self.ReceiveTick`
  (params (DeltaSeconds :type "Float (single-precision)"))
  (bind _returnvalue_location (`KismetMathLibrary.BreakTransform` (`self.GetTransform`)))
  (`self.K2_AddActorLocalRotation` (struct :`Yaw` 5.0))
  (if (`self.Magnet`)
    (`self.K2_SetActorLocation` (`KismetMathLibrary.VInterpTo` _returnvalue_location (`self.K2_GetActorLocation` (`GameplayStatics.GetPlayerCharacter` 0)) (`GameplayStatics.GetWorldDeltaSeconds`) 10.0))))

(event `self.Magnet zone.OnComponentBeginOverlap`
  (params (OverlappedComponent :type "PrimitiveComponent Object Reference") (OtherActor :type "Actor Object Reference") (OtherComp :type "PrimitiveComponent Object Reference") (OtherBodyIndex :type Integer) (bFromSweep :type Boolean) (SweepResult :type "HitResult Structure (by ref)"))
  (cast `/Game/Main/Blueprints/BP_TopDownCharacter` OtherActor)
  (set `self.Magnet` true))

(event `self.Magnet zone.OnComponentEndOverlap`
  (params (OverlappedComponent :type "PrimitiveComponent Object Reference") (OtherActor :type "Actor Object Reference") (OtherComp :type "PrimitiveComponent Object Reference") (OtherBodyIndex :type Integer))
  (cast `/Game/Main/Blueprints/BP_TopDownCharacter` OtherActor)
  (set `self.Magnet` false))

(fn `UserConstructionScript`)