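; BP_Boss is a boss enemy that chases the player and damages them on contact with its Box, throttled by a DoOnce.
; Bullets hitting its capsule subtract their damage from BossHealth, which starts at MaxBossHealth.
; Tick polls for death, then destroys the boss, drops a coin, resets the first enemy spawner's boss state and raises its spawn cap.
; MaxBossHealth is raised only on the dying instance.
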(event `Enemy movement`
  ; Enemy movement
  (`|AIMoveTo` self (0.0 0.0 0.0) (`GameplayStatics.GetPlayerCharacter` 0) :!label _label
    (:`then`
      (`KismetSystemLibrary.Delay` 1.0)
      (goto _label))))

(event `self.ReceiveBeginPlay`
  (`self.Enemy movement`))

(event `Destroy Enemy`
  ; Kill enemy
  (if (<= (`self.Boss_Health`) 0)
    (`self.K2_DestroyActor`)
    (`|SpawnActorFromClass` "/Game/Main/Blueprints/Colletables/BP_Coin.BP_Coin_C" (`self.GetTransform`) "Undefined" "MultiplyWithRoot" null null)
    (bind _outactors (`GameplayStatics.GetAllActorsOfClass` "/Game/Main/Blueprints/Enemies/BP_Enemy_Spawner.BP_Enemy_Spawner_C"))
    (bind _output (`|GetArrayItem` _outactors))
    (set `/Game/Main/Blueprints/Enemies/BP_Enemy_Spawner.Bossspawned` false _output)
    (set `/Game/Main/Blueprints/Enemies/BP_Enemy_Spawner.Enemies_killed` 0.0 _output)
    (set `/Game/Main/Blueprints/Enemies/BP_Enemy_Spawner.Max_enemies_spawn` (+ (`/Game/Main/Blueprints/Enemies/BP_Enemy_Spawner.Max_enemies_spawn` _output) 10.0) _output)
    (set `self.Max_Boss_Health` (+ (`self.Max_Boss_Health`) 50))))

(event `self.ReceiveTick`
  (params (DeltaSeconds :type "Float (single-precision)"))
  (`self.Destroy Enemy`))

(event `self.Box.OnComponentBeginOverlap`
  (params (OverlappedComponent :type "PrimitiveComponent Object Reference") (OtherActor :type "Actor Object Reference") (OtherComp :type "PrimitiveComponent Object Reference") (OtherBodyIndex :type Integer) (bFromSweep :type Boolean) (SweepResult :type "HitResult Structure (by ref)"))
  ; attack player
  (bind _asbp_top_down_character (cast `/Game/Main/Blueprints/BP_TopDownCharacter` OtherActor))
  (`/Engine/EditorBlueprintResources/StandardMacros.DoOnce` false :!label _label_2
    (:`Completed`
      (set `/Game/Main/Blueprints/BP_TopDownCharacter.Player_Health ` (- (`/Game/Main/Blueprints/BP_TopDownCharacter.Player_Health ` _asbp_top_down_character) 50.0) _asbp_top_down_character)
      (`KismetSystemLibrary.Delay` 0.5)
      (goto _label_2 :!via `Reset`))))

(event `self.CapsuleComponent.OnComponentBeginOverlap`
  (params (OverlappedComponent :type "PrimitiveComponent Object Reference") (OtherActor :type "Actor Object Reference") (OtherComp :type "PrimitiveComponent Object Reference") (OtherBodyIndex :type Integer) (bFromSweep :type Boolean) (SweepResult :type "HitResult Structure (by ref)"))
  (bind _asbp_bullet (cast `/Game/Main/Blueprints/BP_Bullet` OtherActor))
  (set `self.Boss_Health` (- (`self.Boss_Health`) (`/Game/Main/Blueprints/BP_Bullet.Damage` _asbp_bullet)))
  (`self.K2_DestroyActor` _asbp_bullet))

(fn `UserConstructionScript`
  (set `self.Boss_Health` (`self.Max_Boss_Health`)))