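; BP_Enemy_Spawner runs wave-based enemy and boss spawning at random reachable navmesh points around the player character.
; A looping timer spawns enemies up to the wave quota, with health scaled by wave number.
; Tick checks when kills equal the quota, then clears remaining enemies and spawns one wave-scaled boss.
; IncreaseWave advances the wave, raises the quota and resets only the spawned count.
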(event `self.ReceiveBeginPlay`
  ; Spawn Enemies
  (`KismetSystemLibrary.K2_SetTimerDelegate` (delegate `Spawn Enemy`) 0.5 true))

(event `Spawn Enemy`
  ; Spawn Enemies
  (if (not (or (`self.Bossspawned`) (== (`self.Max_enemies_spawn`) (`self.Enemies_Spawned`))))
    (bind _asbp_top_down_character (cast `/Game/Main/Blueprints/BP_TopDownCharacter` (`GameplayStatics.GetPlayerCharacter` 0)))
    (bind _returnvalue (`|SpawnActorFromClass` "/Game/Main/Blueprints/Enemies/BP_Enemy.BP_Enemy_C" (`KismetMathLibrary.MakeTransform` (`NavigationSystemV1.K2_GetRandomReachablePointInRadius` (`self.K2_GetActorLocation` _asbp_top_down_character) 7000.0 null null)) "Undefined" "MultiplyWithRoot" null null))
    (set `/Game/Main/Blueprints/Enemies/BP_Enemy.Enemy_Health` (+ (`/Game/Main/Blueprints/Enemies/BP_Enemy.Enemy_Health` _returnvalue) (* (`self.Wave`) 10)) _returnvalue)
    (`/Engine/EditorBlueprintResources/StandardMacros.IncrementFloat` (`self.Enemies_Spawned`))))

(event `SpawnBoss`
  ; Boss Spawning
  (if (== (`self.Max_enemies_spawn`) (`self.Enemies_killed`))
    (bind _outactors (`GameplayStatics.GetAllActorsOfClass` "/Game/Main/Blueprints/Enemies/BP_Enemy.BP_Enemy_C"))
    (`self.K2_DestroyActor` _outactors)
    (if (not (`self.Bossspawned`))
      (bind _asbp_top_down_character (cast `/Game/Main/Blueprints/BP_TopDownCharacter` (`GameplayStatics.GetPlayerCharacter` 0)))
      (bind _returnvalue (`|SpawnActorFromClass` "/Game/Main/Blueprints/Enemies/BP_Boss.BP_Boss_C" (`KismetMathLibrary.MakeTransform` (`NavigationSystemV1.K2_GetRandomReachablePointInRadius` (`self.K2_GetActorLocation` _asbp_top_down_character) 7000.0 null null)) "Undefined" "MultiplyWithRoot" null null))
      (set `/Game/Main/Blueprints/Enemies/BP_Boss.Max_Boss_Health` (+ (`/Game/Main/Blueprints/Enemies/BP_Boss.Max_Boss_Health` _returnvalue) (* (`self.Wave`) 10)) _returnvalue)
      (set `/Game/Main/Blueprints/Enemies/BP_Boss.Boss_Health` (+ (`/Game/Main/Blueprints/Enemies/BP_Boss.Boss_Health` _returnvalue) (* (`self.Wave`) 10)) _returnvalue)
      (set `self.Bossspawned` true))))

(event `self.ReceiveTick`
  (params (DeltaSeconds :type "Float (single-precision)"))
  ; Boss Spawning
  (`self.SpawnBoss`))

(event `Increase Wave`
  ; Increase wave
  (`/Engine/EditorBlueprintResources/StandardMacros.IncrementInt` (`self.Wave`)
    (:`  `
      (set `self.Max_enemies_spawn` (+ (`self.Max_enemies_spawn`) 10.0))
      (set `self.Enemies_Spawned` 0.0))))

(fn `UserConstructionScript`)